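; BP_waveMaster spawns waves of enemies on a repeating timer that starts at BeginPlay.
; Each wave reads its spawn count from the EnemyNumber array, indexed by WaveNumber, then increments WaveNumber with no bounds check.
; Every EnemyTest pawn spawns through SpawnAIFromClass at a randomly picked BP_SpawnLocations actor, with that actor list gathered again on each loop iteration.
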(event Custom|SpawnWave
  (for _index (range 0 (Utilities|Array|Get(acopy) (Variables|Default|GetEnemyNumber) (Variables|Default|GetWaveNumber)))
    (bind _outactors (Actor|GetAllActorsOfClass "/Game/BP_SpawnLocations.BP_SpawnLocations_C"))
    (Variables|Default|SetRandSpawnLocations _outactors)
    (AI|SpawnAIFromClass "/Game/EnemiesAndAI/EnemyTest.EnemyTest_C" 0 (Transformation|GetActorLocation (.OutItem (Utilities|Array|Random (Variables|Default|GetRandSpawnLocations)))) "0, 0, 0" false 0))
  (Math|Integer|IncrementInt (Variables|Default|GetWaveNumber)))

(event EventBeginPlay
  (Utilities|Time|SetTimerbyEvent (delegate Custom|SpawnWave) 15.0 true))

(fn ConstructionScript)